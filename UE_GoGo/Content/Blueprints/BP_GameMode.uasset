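; BP_GameMode is a game mode Blueprint with a PlayerDied event that respawns the dead character by calling RestartPlayer on its controller.
; BeginPlay, Tick and the construction script are empty.
; Disconnected nodes would reset PlayTime, bind PlayerDied to OnPlayerDied, and create the start countdown, timer and game judge widgets.
; As wired, that setup never runs, so this graph neither binds the death event nor shows those widgets.
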(event Custom|Player%20Died
  (params (startCharacter :type Character%20Object%20Reference))
  (Class|GameModeBase|RestartPlayer (Pawn|GetController startCharacter)))

(event EventBeginPlay)

(event EventTick
  (params (DeltaSeconds :type Float%20%28single-precision%29)))

(fn ConstructionScript)