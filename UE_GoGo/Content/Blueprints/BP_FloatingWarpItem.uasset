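; BP_FloatingWarpItem is a pickup that lifts the first-person player upward and then restarts them.
; On overlap with BP_FPCharacter, it destroys its sphere and collision, stores the character and disables their movement.
; While hit, Tick raises the character each frame, scaling FloatingDistance by delta time.
; After a RestartTime delay, it calls the character's RestratPlayer and destroys itself.
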(event OnComponentBeginOverlap(SphereCollision)
  (params (OverlappedComponent :type Primitive%20Component%20Object%20Reference) (OtherActor :type Actor%20Object%20Reference) (OtherComp :type Primitive%20Component%20Object%20Reference) (OtherBodyIndex :type Integer) (bFromSweep :type Boolean) (SweepResult :type Hit%20Result%20Structure%20%28by%20ref%29))
  (bind _asbp_fpcharacter (Utilities|Casting|CastToBP_FPCharacter OtherActor)
    (:then
      (bind _output_get (Variables|Default|SetFPCharacter _asbp_fpcharacter))
      (Components|DestroyComponent (Variables|Default|GetSphere))
      (Components|DestroyComponent (Variables|Default|GetSphere%20Collision))
      (Variables|Default|Setis%20Hit true)
      (Pawn|Components|CharacterMovement|DisableMovement (Variables|/Script/Engine.Character|GetCharacterMovement _output_get))
      (Utilities|FlowControl|Delay (Variables|Default|GetRestart%20Time))
      (Default|RestratPlayer _output_get)
      (Actor|DestroyActor))
    (:CastFailed
      (Development|PrintString "Cast to BP_FPCharacter FAILED"))))

(event EventBeginPlay)

(event Collision|EventActorBeginOverlap
  (params (OtherActor :type Actor%20Object%20Reference)))

(event EventTick
  (params (DeltaSeconds :type Float%20%28single-precision%29))
  (bind _fpcharacter (Variables|Default|GetFPCharacter))
  (if (Variables|Default|Getis%20Hit)
    (Utilities|IsValid _fpcharacter
      (:Is%20Valid
        (Transformation|SetActorLocation _fpcharacter (+ (Math|Vector|MakeVector 0.0 0.0 (* DeltaSeconds (Variables|Default|Getfloating%20Distance))) (Transformation|GetActorLocation _fpcharacter)) false false)))))

(fn ConstructionScript)